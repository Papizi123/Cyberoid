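; Example lightning actor that keeps a permanent Niagara electric arc running between its Start and End components.
; BeginPlay spawns the main arc on Start, and Tick refreshes its end position from End.
; Tick also spawns short curved arcs after random delays scaled by LightningFrequency, randomizing width, brightness and blue-leaning color.
; A zero-delay event loop keeps the latest curved arc's endpoint updated while valid; the movement timeline is disconnected.
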(event Custom|UpdateUserEnd
  (bind _end (Variables|Default|GetEnd))
  (bind _returnvalue (Transformation|GetWorldLocation _end))
  ;[1 1 1] Add lightning effect
  (Class|NiagaraComponent|SetVariablePosition (stale EventTick _returnvalue_2) "User.EndPos" _returnvalue)
  (Effects|Components|ParticleSystem|SetVectorParameter (stale EventTick _returnvalue_2) "User.End" _returnvalue)
  (Utilities|FlowControl|Delay 0.0)
  (Utilities|IsValid (stale EventTick _returnvalue_2)
    (:Is%20Valid
      (CallFunction|UpdateUserEnd))))

(event EventBeginPlay
  ;[1 1 1] Add lightning effect
  (bind _returnvalue (Niagara|SpawnSystemAttached "/Game/Lightning_Electricity_Pack/Particles/V1_25/P_PermanentArc1.P_PermanentArc1" (Variables|Default|GetStart) "None" "0, 0, 0" "0, 0, 0" "KeepRelativeOffset" true))
  (bind _output_get (Variables|Default|SetElectricArc _returnvalue))
  (Class|NiagaraComponent|SetVariablePosition _output_get "User.EndPos" (Transformation|GetWorldLocation (Variables|Default|GetEnd))))

(event EventTick
  (params (DeltaSeconds :type Float%20%28single-precision%29))
  (bind _electricarc (Variables|Default|GetElectricArc))
  (bind _end (Variables|Default|GetEnd))
  (bind _returnvalue (Transformation|GetWorldLocation _end))
  (Utilities|FlowControl|Sequence
    (:then_0
      ;[1 1 1] Add lightning effect
      (Utilities|FlowControl|Delay (* (Math|Random|RandomFloatinRange 1.0 3.0) (Variables|Default|GetLightningFrequency)))
      (bind _returnvalue_2 (Niagara|SpawnSystemAttached "/Game/Lightning_Electricity_Pack/Particles/V1_25/P_curved_Arcs.P_curved_Arcs" (Variables|Default|GetStart) "None" "0, 0, 0" "0, 0, 0" "KeepRelativeOffset" true))
      (Effects|Components|ParticleSystem|SetFloatParameter _returnvalue_2 "User.RibbonWidth" (Math|Random|RandomFloatinRange 0.75 1.1))
      (Effects|Components|ParticleSystem|SetFloatParameter _returnvalue_2 "User.MinLifeTime" 0.25)
      (Effects|Components|ParticleSystem|SetFloatParameter _returnvalue_2 "User.MaxLifeTime" 0.35)
      (Effects|Components|ParticleSystem|SetFloatParameter _returnvalue_2 "User.ColorBoost" (Math|Random|RandomFloatinRange 2e+01 5e+01))
      (Effects|Components|ParticleSystem|SetColorParameter _returnvalue_2 "User.Color" (Utilities|Struct|MakeLinearColor (Math|Random|RandomFloatinRange 0.0 0.4) (Math|Random|RandomFloatinRange 0.25 0.65) (Math|Random|RandomFloatinRange 0.65 1.0) 1.0))
      (Class|NiagaraComponent|SetVariablePosition _returnvalue_2 "User.EndPos" _returnvalue)
      (Effects|Components|ParticleSystem|SetVectorParameter _returnvalue_2 "User.End" _returnvalue)
      (Utilities|FlowControl|Delay 0.0)
      (Utilities|IsValid _returnvalue_2
        (:Is%20Valid
          (CallFunction|UpdateUserEnd))))
    (:then_1
      ;[1 1 1] Update User.End
      (Utilities|IsValid _electricarc
        (:Is%20Valid
          (Class|NiagaraComponent|SetVariablePosition _electricarc "User.EndPos" (Transformation|GetWorldLocation (Variables|Default|GetEnd))))))))

(fn ConstructionScript)