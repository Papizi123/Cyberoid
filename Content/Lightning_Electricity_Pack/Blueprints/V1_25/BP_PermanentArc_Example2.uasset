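; Example Blueprint from a lightning effects pack that displays a permanent electric arc between its Start and End components.
; BeginPlay spawns the P_PermanentArc2 Niagara system attached to Start and passes End's world location to its User.EndPos parameter.
; Tick refreshes that endpoint while the arc is valid, so it follows End.
; A movement timeline and older User.End setters remain in the graph but never run.
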(event EventBeginPlay
  ;[1 1 1] Add lightning effect
  (bind _returnvalue (Niagara|SpawnSystemAttached "/Game/Lightning_Electricity_Pack/Particles/V1_25/P_PermanentArc2.P_PermanentArc2" (Variables|Default|GetStart) "None" "0, 0, 0" "0, 0, 0" "KeepRelativeOffset" true))
  (bind _output_get (Variables|Default|SetElectricArc _returnvalue))
  (Class|NiagaraComponent|SetVariablePosition _output_get "User.EndPos" (Transformation|GetWorldLocation (Variables|Default|GetEnd))))

(event EventTick
  (params (DeltaSeconds :type Float%20%28single-precision%29))
  (bind _electricarc (Variables|Default|GetElectricArc))
  ;[1 1 1] Update User.End
  (Utilities|IsValid _electricarc
    (:Is%20Valid
      (Class|NiagaraComponent|SetVariablePosition _electricarc "User.EndPos" (Transformation|GetWorldLocation (Variables|Default|GetEnd))))))

(fn ConstructionScript)