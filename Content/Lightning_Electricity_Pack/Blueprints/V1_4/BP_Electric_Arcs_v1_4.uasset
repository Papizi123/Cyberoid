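; Lightning pack effect actor that plays a repeating electric arc sequence, starting half a second after BeginPlay.
; A timeline scales the Energy particle system through its size user parameter and moves it vertically relative to the actor's location.
; Alongside it, delays switch the Arcs effect on shortly after each cycle starts and off a few seconds later.
; When the timeline finishes, the Again event restarts the cycle after a short pause.
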(event Custom|Again
  (bind _energy (Variables|Default|GetEnergy))
  (bind _arcs (Variables|Default|GetArcs))
  (Utilities|FlowControl|Sequence
    (:then_0
      (bind (_direction _scale _z_offset) (Timeline|Timeline PlayFromStart)
        (:Update
          (Utilities|FlowControl|Sequence
            (:then_0
              (if (Components|Activation|IsActive _energy)
                (Effects|Components|ParticleSystem|SetFloatParameter _energy "User.System_Size" _scale)))
            (:then_1
              (Transformation|SetWorldLocation _energy (+ (Math|Vector|MakeVector 0.0 0.0 (* _z_offset 4e+02)) (Transformation|GetActorLocation)) false true))))
        (:Finished
          (Utilities|FlowControl|Delay 1.0)
          (CallFunction|Again))))
    (:then_1
      (Utilities|FlowControl|Delay 0.25)
      (Components|Activation|Activate _arcs true)
      (Utilities|FlowControl|Delay 4.25)
      (Components|Activation|Deactivate _arcs))))

(event EventBeginPlay
  (bind _energy (Variables|Default|GetEnergy))
  (bind _arcs (Variables|Default|GetArcs))
  (Utilities|FlowControl|Delay 0.5)
  (Utilities|FlowControl|Sequence
    (:then_0
      (bind (_direction _scale _z_offset) (Timeline|Timeline PlayFromStart)
        (:Update
          (Utilities|FlowControl|Sequence
            (:then_0
              (if (Components|Activation|IsActive _energy)
                (Effects|Components|ParticleSystem|SetFloatParameter _energy "User.System_Size" _scale)))
            (:then_1
              (Transformation|SetWorldLocation _energy (+ (Math|Vector|MakeVector 0.0 0.0 (* _z_offset 4e+02)) (Transformation|GetActorLocation)) false true))))
        (:Finished
          (Utilities|FlowControl|Delay 1.0)
          (CallFunction|Again))))
    (:then_1
      (Utilities|FlowControl|Delay 0.25)
      (Components|Activation|Activate _arcs true)
      (Utilities|FlowControl|Delay 4.25)
      (Components|Activation|Deactivate _arcs))))

(fn ConstructionScript)