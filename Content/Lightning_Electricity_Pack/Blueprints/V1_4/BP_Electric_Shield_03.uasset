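; Electric shield effect actor that loops a Niagara shield on and off, apparently for showcasing the effect.
; After an initial delay it activates the Electricity component and sets its size and color parameters.
; Timelines then flash the color toward a hit tint and shrink the shield before deactivating it, and the cycle repeats after a pause.
; A movement timeline that would offset and rotate the actor is present but never runs.
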(event Custom|Shield
  (bind _electricity (Variables|Default|GetElectricity))
  ;[1 1 1] Activate
  (Components|Activation|Activate _electricity true)
  (Effects|Components|ParticleSystem|SetFloatParameter _electricity "User.Deactivate_Size" 1.0)
  (Effects|Components|ParticleSystem|SetColorParameter _electricity "User.Shield_Color" (Variables|Default|GetShield_Color))
  (Utilities|FlowControl|Sequence
    (:then_0
      (Utilities|FlowControl|Delay 4.0)
      ;[1 1 1] Deactivate
      (bind _deactivate_size (Timeline|Timeline_1 PlayFromStart)
        (:Update
          (Effects|Components|ParticleSystem|SetFloatParameter (Variables|Default|GetElectricity) "User.Deactivate_Size" _deactivate_size))
        (:Finished
          (Components|Activation|Deactivate _electricity)
          (Utilities|FlowControl|Delay 1e+01)
          (CallFunction|Shield))))
    (:then_1
      ;[1 1 1] Hit
      (Utilities|FlowControl|Delay 3.0)
      (bind _hit (Timeline|Color_Hit PlayFromStart)
        (:Update
          (Effects|Components|ParticleSystem|SetColorParameter _electricity "User.Shield_Color" (Math|Color|Lerp(LinearColor) (Variables|Default|GetShield_Color) (Variables|Default|GetShield_Color_Hit) _hit)))))))

(event EventBeginPlay
  (Variables|Default|SetStartLocation (Transformation|GetActorLocation))
  (Utilities|FlowControl|Delay (Variables|Default|GetFirstDelay))
  (CallFunction|Shield))

(fn ConstructionScript)